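; Base enemy AI character that chases and melee-attacks the ninja player, with health bar, hit reactions and death cleanup.
; Move runs a self-repeating AIMoveTo loop while the player is alive, turning and playing the attack montage on arrival.
; EnemyExecution line-traces forward for pawns, then either plays a block sound or applies damage.
; The Health component feeds the widget and triggers death animation, collision shutdown and delayed destruction.
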(event `self.ReceiveAnyDamage`
  (params (Damage :type "Float (single-precision)") (DamageType :type "DamageType Object Reference") (InstigatedBy :type "Controller Object Reference") (DamageCauser :type "Actor Object Reference"))
  ; Damage
  (`parent.ReceiveAnyDamage` Damage DamageType InstigatedBy DamageCauser)
  (`self.PlayAnimMontage` "/Game/NinjaGame/MyNinja/Animations/Main_Anim/Enemy/AM_Enemy_React.AM_Enemy_React")
  (`KismetSystemLibrary.Delay` 0.2)
  (`GameplayStatics.PlaySound2D` "/Game/NinjaGame/MyNinja/Sound/MainCharDamage/EnemyDamage.EnemyDamage" 1.0 1.0 0.0 null null))

(event `self.Health.OnDeath`
  ; Death
  (`PrimitiveComponent.SetCollisionEnabled` (`self.CapsuleComponent`) "NoCollision")
  (`SkeletalMeshComponent.PlayAnimation` (`self.Mesh`) "/Game/NinjaGame/MyNinja/Animations/Main_Anim/Enemy/A_Enemy_Death.A_Enemy_Death" false)
  (`PrimitiveComponent.SetCollisionEnabled` (`self.Mesh`) "NoCollision")
  (`KismetSystemLibrary.Delay` 7.0)
  (`self.K2_DestroyActor`))

(event `EnemyExecution`
  (bind _returnvalue (`self.K2_GetActorLocation`))
  ;[0.15 0.1009 0.09496 0.5] Attack
  (bind _outhit (`KismetSystemLibrary.LineTraceSingleForObjects` _returnvalue (+ _returnvalue (* (`self.GetActorForwardVector`) (`self.AttackDistance`))) (`|MakeArray` "ObjectTypeQuery3" :!type "EObjectTypeQuery Enum")))
  (bind _yes (`self.BlockedAttack` (`.HitActor` (`GameplayStatics.BreakHitResult` _outhit))))
  (if _yes
    (`KismetSystemLibrary.Delay` 0.8)
    (`GameplayStatics.PlaySound2D` "/Game/NinjaGame/MyNinja/Sound/AttackBlock/player_block_Cue.player_block_Cue" 1.0 1.0 0.0 null null)
    (else
      (`GameplayStatics.ApplyDamage` (`.HitActor` (`GameplayStatics.BreakHitResult` _outhit)) (`self.GetDamage`)))))

(event `self.ReceiveBeginPlay`
  ; AI
  (set `self.TeamPlayer` 1) ; All enemies go to 1 group
  ;;[0.008429 0.15 0.08085 0.5] EnemyHealthBar
  (bind _asui_enemy_health (cast `/Game/NinjaGame/MyNinja/UI/EnemyUI/UI_Enemy_Health` (`WidgetComponent.GetUserWidgetObject` (`self.EnemyHealthBarWidget`))))
  (`/Game/NinjaGame/MyNinja/UI/EnemyUI/UI_Enemy_Health.SetHealthComponent` _asui_enemy_health (`self.Health`)))

(event `Move`
  ; AI
  (bind _asbp_ninja_player (cast `/Game/NinjaGame/MyNinja/Character/Ninja/BP_NinjaPlayer` (`GameplayStatics.GetPlayerCharacter` 0)))
  ;; Странная тема, я обходил баг, выглядит криво, переделаю
  (if (> (`HealthComponent.Health` (`/Game/NinjaGame/MyNinja/Character/Ninja/BP_NinjaPlayer.Health` _asbp_ninja_player)) 0.0)
    (if (not (<= (`HealthComponent.Health` (`/Game/NinjaGame/MyNinja/Character/Ninja/BP_NinjaPlayer.Health` _asbp_ninja_player)) 0.0))
      (`|AIMoveTo` self (0.0 0.0 0.0) (`GameplayStatics.GetPlayerController` 0) 100.0
        (:`OnSuccess`
          (`self.K2_SetActorRotation` (`self.GetNewRotation`))
          (`self.PlayAnimMontage` "/Game/NinjaGame/MyNinja/Animations/Main_Anim/Enemy/A_Enemy_Attack.A_Enemy_Attack")
          (`KismetSystemLibrary.Delay` 0.2))
        (:`OnFail`
          _))
      (`self.Move`))))

(fn `GetNewRotation`
  (returns (NewParam :type "Rotator Structure"))
  (return (`KismetMathLibrary.FindLookAtRotation` (`self.K2_GetActorLocation`) (`self.K2_GetActorLocation` (`GameplayStatics.GetPlayerCharacter` 0)))))

(fn `UserConstructionScript`
  (`parent.UserConstructionScript`))